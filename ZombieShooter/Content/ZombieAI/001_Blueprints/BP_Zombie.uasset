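; Zombie enemy Blueprint that patrols, chases pawns it sees and attacks them in melee.
; Patrol uses AI MoveTo to random reachable points, retrying on failure but stopping after a short delay on success.
; PawnSensing triggers the chase, which plays a CanAttack-gated montage on arrival or returns to patrol on failure.
; A montage notify runs a debug-drawn sphere trace for damage, its end multiplying location by the forward offset rather than adding it.
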(event OnSeePawn(PawnSensing)
  (params (Pawn :type Pawn%20Object%20Reference))
  (CallFunction|ChaseTarget Pawn))

(event Custom|Patrol
  (AI|AIMoveTo self (.RandomLocation (AI|Navigation|GetRandomReachablePointinRadius (Transformation|GetActorLocation) 2.5e+03 0 0)) 0 5.0 false
    (:OnSuccess
      (Utilities|FlowControl|Delay 0.8))
    (:OnFail
      (CallFunction|Patrol))))

(event Custom|Chase%20Target
  (params (TargetActor :type Actor%20Object%20Reference))
  (bind _returnvalue (Transformation|GetActorLocation))
  (AI|AIMoveTo self "0, 0, 0" TargetActor 1.2e+02 false
    (:OnSuccess
      (if (Variables|Default|GetCanAttack?)
        (Animation|Montage|PlayMontage (Variables|Character|GetMesh) 0
          (:then
            (Variables|Default|SetCanAttack? false))
          (:OnCompleted
            (Variables|Default|SetCanAttack? true :!label _label))
          (:OnInterrupted
            (goto _label))
          (:OnNotifyBegin
            (bind (_outhit _returnvalue_2) (Collision|SphereTraceForObjects _returnvalue (* _returnvalue (* (Math|Vector|GetForwardVector (Transformation|GetActorRotation)) 2e+02)) 0.0 (Utilities|Array|MakeArray "ObjectTypeQuery3") false 0 "ForDuration" true "(R=1.000000,G=0.000000,B=0.000000,A=1.000000)" "(R=0.000000,G=1.000000,B=0.000000,A=1.000000)" 0.5))
            (if _returnvalue_2
              (Game|Damage|ApplyDamage (.HitActor (Collision|BreakHitResult _outhit)) 2e+01 0 0))))))
    (:OnFail
      (CallFunction|Patrol))))

(event EventBeginPlay
  (CallFunction|Patrol))

(fn ConstructionScript)